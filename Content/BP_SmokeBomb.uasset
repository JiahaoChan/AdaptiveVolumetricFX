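; BP_SmokeBomb is a smoke bomb Blueprint that builds its explosion volume from instanced meshes.
; ExplodewithAnim clears the MeshComponent instances at layer zero, then adds a world-space instance for each node in that ExplodeLayers entry.
; It calls itself recursively on the next layer until the index is invalid, with no delay between layers despite the animation in its name.
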(event `self.ExplodeWithAnim`
  (params (LayerIndex :type Integer))
  (bind _explodelayers (`self.ExplodeLayers`))
  (`|ExecutionSequence`
    (:`then_0`
      (if (== LayerIndex 0)
        (`InstancedStaticMeshComponent.ClearInstances` (`self.MeshComponent`))))
    (:`then_1`
      (if (`KismetArrayLibrary.Array_IsValidIndex` _explodelayers LayerIndex)
        (for _array_element (`.Nodes` (break `ExplodeLayer` (`|GetArrayItem` _explodelayers LayerIndex)))
          (`InstancedStaticMeshComponent.AddInstance` (`self.MeshComponent`) (`KismetMathLibrary.MakeTransform` _array_element) true))
        (`self.ExplodeWithAnim` (+ LayerIndex 1))))))

(fn `UserConstructionScript`)